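; Straight level template for Crimson Maze that spawns one random enemy at its EnemySpawn point.
; The construction script runs the parent's, then uses nested random rolls to favor sword and ranged daemons over the rarer drone.
; Each spawn event creates its enemy class and gives it a default controller.
; A short delay precedes each spawn as a workaround, since spawning straight from the construction script fails.
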(event Custom|SpawnSimpleRangeDaemon
  ;[1 1 1] Spawn Enemy
  (Utilities|FlowControl|Delay 0.1) ; Ohne Delay funktioniert es nicht. \nVllt wird spawnactor zu früh aufgerufen, weil es über das constructuin script läuft
  (bind _returnvalue (Game|SpawnActorfromClass "/Game/CrimsonMaze/Core/Enemies/BP_SimpleRangeDaemon.BP_SimpleRangeDaemon_C" (Math|Transform|MakeTransform (Transformation|GetWorldLocation (Variables|Default|GetEnemySpawn)) "0, 0, 0" "1,1,1") "Undefined" 0 0))
  (Pawn|SpawnDefaultController _returnvalue))

(event Custom|SpawnDrone
  ;[1 1 1] Spawn Enemy
  (Utilities|FlowControl|Delay 0.1) ; Ohne Delay funktioniert es nicht. \nVllt wird spawnactor zu früh aufgerufen, weil es über das constructuin script läuft
  (bind _returnvalue (Game|SpawnActorfromClass "/Game/CrimsonMaze/Core/Enemies/BP_EnemyDrone.BP_EnemyDrone_C" (Math|Transform|MakeTransform (Transformation|GetWorldLocation (Variables|Default|GetEnemySpawn)) "0, 0, 0" "1,1,1") "Undefined" 0 0))
  (Pawn|SpawnDefaultController _returnvalue))

(event Custom|SpawnSimpleSowrdDaemon
  ;[1 1 1] Spawn Enemy
  (Utilities|FlowControl|Delay 0.1) ; Ohne Delay funktioniert es nicht. \nVllt wird spawnactor zu früh aufgerufen, weil es über das constructuin script läuft
  (bind _returnvalue (Game|SpawnActorfromClass "/Game/CrimsonMaze/Core/Enemies/BP_SimpleSwordDaemon.BP_SimpleSwordDaemon_C" (Math|Transform|MakeTransform (Transformation|GetWorldLocation (Variables|Default|GetEnemySpawn)) "0, 0, 0" "1,1,1") "Undefined" 0 0))
  (Pawn|SpawnDefaultController _returnvalue))

(fn ConstructionScript
  (|CallParentFunction)
  (switch int (Math|Random|RandomInteger 3)
    (:0
      (switch int (Math|Random|RandomInteger 3)
        (:0
          (CallFunction|SpawnDrone))
        (:1
          (CallFunction|SpawnSimpleSowrdDaemon))
        (:2
          (CallFunction|SpawnSimpleRangeDaemon))))
    (:1
      (CallFunction|SpawnSimpleSowrdDaemon))
    (:2
      (CallFunction|SpawnSimpleRangeDaemon))))