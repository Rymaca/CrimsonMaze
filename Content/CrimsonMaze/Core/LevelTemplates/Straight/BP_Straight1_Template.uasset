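; Straight level template for Crimson Maze, drafted to randomly place an obstacle, though that logic is currently disconnected.
; The construction script only calls its parent; the unwired setup selects a rock, falling wreckage trigger, sword daemon or ranged daemon.
; Unwired event logic would spawn daemons with controllers after a delay, or reveal wreckage and lerp it to a target by timeline.
; The trigger and custom events are empty.
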(event OnComponentBeginOverlap(FallingWreckageTrigger)
  (params (OverlappedComponent :type Primitive%20Component%20Object%20Reference) (OtherActor :type Actor%20Object%20Reference) (OtherComp :type Primitive%20Component%20Object%20Reference) (OtherBodyIndex :type Integer) (bFromSweep :type Boolean) (SweepResult :type Hit%20Result%20Structure%20%28by%20ref%29))
  ;[0.6344 0.3297 0.3601] Falling Wreckage Zeugs
)

(event Custom|Falling%20Wreckage%20Event
  ;[0.6344 0.3297 0.3601] Falling Wreckage Zeugs
)

(event Custom|SpawnSimpleRangeDaemon
  ;[1 1 1] Spawn Enemy
)

(event Custom|SpawnSimpleSowrdDaemon
  ;[1 1 1] Spawn Enemy
)

(fn ConstructionScript
  (|CallParentFunction))

(fn SetVisibilityandCollision(FallingWreckage)
  (bind _fallingwreckage (Variables|Default|GetFallingWreckage))
  (Rendering|SetVisibility _fallingwreckage true false)
  (Variables|/Script/Engine.PrimitiveComponent|SetbGenerateOverlapEvents _fallingwreckage false)
  (Collision|SetCollisionEnabled _fallingwreckage "QueryAndPhysics"))