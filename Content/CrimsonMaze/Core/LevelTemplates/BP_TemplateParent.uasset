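; Parent actor for the side-scroller's level templates that endlessly chains randomly chosen straight and branching segments across three lanes.
; Entry overlap spawns straight pieces until a minimum run is met, then a lane-aware random selector picks an allowed template.
; Lane state and spawn flags are copied into each spawned template, and lane triggers adjust their current lane.
; Exit overlap destroys the template, while the fall trigger kills the player.
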(event OnComponentBeginOverlap(EntryCollision)
  (params (OverlappedComponent :type Primitive%20Component%20Object%20Reference) (OtherActor :type Actor%20Object%20Reference) (OtherComp :type Primitive%20Component%20Object%20Reference) (OtherBodyIndex :type Integer) (bFromSweep :type Boolean) (SweepResult :type Hit%20Result%20Structure%20%28by%20ref%29))
  (Utilities|Casting|CastTo2DSideScrollerCharacter OtherActor)
  (Utilities|FlowControl|DoOnce false
    (:Completed
      ;[1 1 1] Damit eine bestimmte Anzahl gerader Lanes kommen muss!
      ; -> Nach Lane Switch muss mindestens eine Gerade kommen, weil nur Gerade an unterschiedlichen Spawnpoints gleichzeitig spawnen können!
      (if (> (Variables|Default|GetMinimumStraightLanesInRow) (Variables|Default|GetStraightLaneCount))
        (CallFunction|SetupSpawnPointsOfStraightTemplates)
        (else
          ;[1 1 1] Richtige Lane ermitteln und eine mögliche Passende Lane dazu spawnen.
          ; Anmerkung: In Spawn Funktionen ist der Spawnpunkt immer "0", weil ja immer eine StraightLane dazwischen ist und die den Spawnpoint0 hat
          (Utilities|DetermineCurrentLane
            (:Lane%201
              (Utilities|SelectLaneReworked :!label _label
                (:Straight
                  (Variables|Default|SetSpawnInLane0 true) ; Ist ein fix, damit nach einer normalen Straight Lane etwas spawnen kann. Also damit zwei normale straight Lanes hintereinander kommen können
                  (CallFunction|SetupSpawnPointsOfStraightTemplates))
                (:Down
                  (CallFunction|SpawnDownTemplate))
                (:Up
                  (CallFunction|SpawnUpTemplate))
                (:Straight%20+%20Down
                  (CallFunction|SpawnStraightandDownTemplate))
                (:Straight%20+%20Up
                  (CallFunction|SpawnStraightandUpTemplate))
                (:Straight%20+%20Up%20+%20Down
                  (CallFunction|SpawnStraightandUpandDownTemplate))
                (:Up%20+%20Down
                  (CallFunction|SpawnUpandDownTemplate))))
            (:Lane%200
              (goto _label Lane%200))
            (:Lane%20-1
              (goto _label Lane%20-1))))))))

(event OnComponentBeginOverlap(ExitCollision)
  (params (OverlappedComponent :type Primitive%20Component%20Object%20Reference) (OtherActor :type Actor%20Object%20Reference) (OtherComp :type Primitive%20Component%20Object%20Reference) (OtherBodyIndex :type Integer) (bFromSweep :type Boolean) (SweepResult :type Hit%20Result%20Structure%20%28by%20ref%29))
  ;[1 1 1] Level template gets destroyed so game won't overload and crash
  (Utilities|Casting|CastTo2DSideScrollerCharacter OtherActor)
  (Actor|DestroyActor))

(event OnComponentBeginOverlap(Lane0Collision)
  (params (OverlappedComponent :type Primitive%20Component%20Object%20Reference) (OtherActor :type Actor%20Object%20Reference) (OtherComp :type Primitive%20Component%20Object%20Reference) (OtherBodyIndex :type Integer) (bFromSweep :type Boolean) (SweepResult :type Hit%20Result%20Structure%20%28by%20ref%29))
  ;[1 1 1] Kontrolle über Lane-Variable. Also damit die Variable der Lane entspricht, auf der der Spieler läuft bzw. wechselt
  (Utilities|Casting|CastTo2DSideScrollerCharacter OtherActor)
  ;;[0.7385 0.7385 0.7385 1 26] -- oder ++ passiert nachdem die Variable weitergegeben wurde. Deshalb wird das nachträglich über das Array weitergegeben
  (Utilities|FlowControl|DoOnce false
    (:Completed
      ;;[1 0.9003 0.2233 1 12] Debug
      (Development|PrintString (Utilities|String|Append "Current Lane: " (Utilities|String|ToString(Integer) (Variables|Default|GetCurrentLane)))))))

(event OnComponentBeginOverlap(Lane1Collision)
  (params (OverlappedComponent :type Primitive%20Component%20Object%20Reference) (OtherActor :type Actor%20Object%20Reference) (OtherComp :type Primitive%20Component%20Object%20Reference) (OtherBodyIndex :type Integer) (bFromSweep :type Boolean) (SweepResult :type Hit%20Result%20Structure%20%28by%20ref%29))
  ;[1 1 1] Kontrolle über Lane-Variable. Also damit die Variable der Lane entspricht, auf der der Spieler läuft bzw. wechselt
  (Utilities|Casting|CastTo2DSideScrollerCharacter OtherActor)
  ;;[0.7385 0.7385 0.7385 1 26] -- oder ++ passiert nachdem die Variable weitergegeben wurde. Deshalb wird das nachträglich über das Array weitergegeben
  (Utilities|FlowControl|DoOnce false
    (:Completed
      (for _array_element (Variables|Default|GetSpawnedTemplatesArray)
        (Math|Integer|IncrementInt (Variables|BP_TemplateParent_C|GetCurrentLane _array_element)
          (:%20%20
            ;;[1 0.9003 0.2233 1 12] Debug
            (Development|PrintString (Utilities|String|Append "Current Lane: " (Utilities|String|ToString(Integer) (Variables|Default|GetCurrentLane))))))))))

(event OnComponentBeginOverlap(Lane-1Collision)
  (params (OverlappedComponent :type Primitive%20Component%20Object%20Reference) (OtherActor :type Actor%20Object%20Reference) (OtherComp :type Primitive%20Component%20Object%20Reference) (OtherBodyIndex :type Integer) (bFromSweep :type Boolean) (SweepResult :type Hit%20Result%20Structure%20%28by%20ref%29))
  ;[1 1 1] Kontrolle über Lane-Variable. Also damit die Variable der Lane entspricht, auf der der Spieler läuft bzw. wechselt
  (Utilities|Casting|CastTo2DSideScrollerCharacter OtherActor)
  ;;[0.7385 0.7385 0.7385 1 26] -- oder ++ passiert nachdem die Variable weitergegeben wurde. Deshalb wird das nachträglich über das Array weitergegeben
  (Utilities|FlowControl|DoOnce false
    (:Completed
      (for _array_element (Variables|Default|GetSpawnedTemplatesArray)
        (Math|Integer|DecrementInt (Variables|BP_TemplateParent_C|GetCurrentLane _array_element)
          (:%20%20
            ;;[1 0.9003 0.2233 1 12] Debug
            (Development|PrintString (Utilities|String|Append "Current Lane: " (Utilities|String|ToString(Integer) (Variables|Default|GetCurrentLane))))))))))

(event OnComponentBeginOverlap(FallToDeathCollision)
  (params (OverlappedComponent :type Primitive%20Component%20Object%20Reference) (OtherActor :type Actor%20Object%20Reference) (OtherComp :type Primitive%20Component%20Object%20Reference) (OtherBodyIndex :type Integer) (bFromSweep :type Boolean) (SweepResult :type Hit%20Result%20Structure%20%28by%20ref%29))
  ;[1 1 1] Runterfallen = Spieler-Tod
  (bind _as2dside_scroller_character (Utilities|Casting|CastTo2DSideScrollerCharacter OtherActor))
  (Default|SpielerErhältSchaden _as2dside_scroller_character 999))

(fn ConstructionScript)

(fn CarryonVariables
  (params (NewTemplate :type BP%20Template%20Parent%20Object%20Reference))
  (Variables|BP_TemplateParent_C|SetCurrentLane NewTemplate (Variables|Default|GetCurrentLane))
  (Variables|BP_TemplateParent_C|SetStraightLaneCount NewTemplate (Variables|Default|GetStraightLaneCount))
  (Variables|BP_TemplateParent_C|SetSpawnInLane1 NewTemplate (Variables|Default|GetSpawnInLane1))
  (Variables|BP_TemplateParent_C|SetSpawnInLane-1 NewTemplate (Variables|Default|GetSpawnInLane-1))
  (Variables|BP_TemplateParent_C|SetSpawnInLane0 NewTemplate (Variables|Default|GetSpawnInLane0)))

(fn AddTemplatetoArrayandCarryonVariables
  (params (SpawnedTemplate :type BP%20Template%20Parent%20Object%20Reference))
  (Utilities|Array|Add (Variables|Default|GetSpawnedTemplatesArray) SpawnedTemplate)
  (CallFunction|CarryonVariables SpawnedTemplate))

(fn SetupSpawnPointsOfStraightTemplates
  ;[1 1 1] Wichtig, damit eine mindest-Anzahl an Straight-Lanes kommt
  (Math|Integer|IncrementInt (Variables|Default|GetStraightLaneCount)
    (:%20%20
      (Utilities|FlowControl|Sequence
        (:then_0
          (if (Variables|Default|GetSpawnInLane0)
            (Variables|Default|SetSpawnInLane0 false)
            (CallFunction|SpawnStraightTemplate (Variables|Default|GetSpawnLocationLane0))))
        (:then_1
          ;[1 1 1] Es soll nur true sein, wenn vorher ein Template mit 2 Wegen war, und nachdem 2 StraightLanes gespawnt wurden, wird die Variable wieder false!
          (if (Variables|Default|GetSpawnInLane1)
            (Variables|Default|SetSpawnInLane1 false)
            (CallFunction|SpawnStraightTemplate (Variables|Default|GetSpawnLocationLane1))))
        (:then_2
          ;[1 1 1] Es soll nur true sein, wenn vorher ein Template mit 3 Wegen war, und nachdem 3 StraightLanes gespawnt wurden, wird die Variable wieder false.
          ; Es ist wichtig, dass die Variable wirlich nur true ist, wenn das explizit gewollt ist
          (if (Variables|Default|GetSpawnInLane-1)
            (Variables|Default|SetSpawnInLane-1 false)
            (CallFunction|SpawnStraightTemplate (Variables|Default|GetSpawnLocationLane-1))))))))

(fn SpawnStraightTemplate
  (params (Spawn%20Location :type Scene%20Component%20Object%20Reference))
  (LocalVariables|SetLocalVarSpawnPoint Spawn%20Location)
  (switch int (Math|Random|RandomInteger 4)
    (:0
      (bind _returnvalue (Game|SpawnActorfromClass "/Game/CrimsonMaze/Core/LevelTemplates/Straight/BP_Straight1Enemy_Template.BP_Straight1Enemy_Template_C" (Math|Transform|MakeTransform (Transformation|GetWorldLocation (LocalVariables|GetLocalVarSpawnPoint)) "0, 0, 0" "1,1,1") "Undefined" 0 0))
      (CallFunction|AddTemplatetoArrayandCarryonVariables _returnvalue))
    (:1
      (bind _returnvalue_2 (Game|SpawnActorfromClass "/Game/CrimsonMaze/Core/LevelTemplates/Straight/BP_Straight1FallingWreckage_Template.BP_Straight1FallingWreckage_Template_C" (Math|Transform|MakeTransform (Transformation|GetWorldLocation (LocalVariables|GetLocalVarSpawnPoint)) "0, 0, 0" "1,1,1") "Undefined" 0 0))
      (CallFunction|AddTemplatetoArrayandCarryonVariables _returnvalue_2))
    (:2
      (bind _returnvalue_3 (Game|SpawnActorfromClass "/Game/CrimsonMaze/Core/LevelTemplates/Straight/BP_Straight1Obstacle_Template.BP_Straight1Obstacle_Template_C" (Math|Transform|MakeTransform (Transformation|GetWorldLocation (LocalVariables|GetLocalVarSpawnPoint)) "0, 0, 0" "1,1,1") "Undefined" 0 0))
      (CallFunction|AddTemplatetoArrayandCarryonVariables _returnvalue_3))
    (:3
      (bind _returnvalue_4 (Game|SpawnActorfromClass "/Game/CrimsonMaze/Core/LevelTemplates/Straight/BP_Straight1_Template.BP_Straight1_Template_C" (Math|Transform|MakeTransform (Transformation|GetWorldLocation (LocalVariables|GetLocalVarSpawnPoint)) "0, 0, 0" "1,1,1") "Undefined" 0 0))
      (CallFunction|AddTemplatetoArrayandCarryonVariables _returnvalue_4))))

(fn SpawnDownTemplate
  (Variables|Default|SetStraightLaneCount 0)
  (Variables|Default|SetSpawnInLane-1 true)
  (switch int (Math|Random|RandomInteger 2)
    (:0
      (bind _returnvalue (Game|SpawnActorfromClass "/Game/CrimsonMaze/Core/LevelTemplates/Down/BP_Down1_Template.BP_Down1_Template_C" (Math|Transform|MakeTransform (Transformation|GetWorldLocation (Variables|Default|GetSpawnLocationLane0)) "0, 0, 0" "1,1,1") "Undefined" 0 0))
      (CallFunction|AddTemplatetoArrayandCarryonVariables _returnvalue))
    (:1
      (bind _returnvalue_2 (Game|SpawnActorfromClass "/Game/CrimsonMaze/Core/LevelTemplates/Down/BP_Down2_Template1.BP_Down2_Template1_C" (Math|Transform|MakeTransform (Transformation|GetWorldLocation (Variables|Default|GetSpawnLocationLane0)) "0, 0, 0" "1,1,1") "Undefined" 0 0))
      (CallFunction|AddTemplatetoArrayandCarryonVariables _returnvalue_2))))

(fn SpawnUpTemplate
  (Variables|Default|SetStraightLaneCount 0)
  (Variables|Default|SetSpawnInLane1 true)
  (switch int (Math|Random|RandomInteger 3)
    (:0
      (bind _returnvalue (Game|SpawnActorfromClass "/Game/CrimsonMaze/Core/LevelTemplates/Up/BP_Up1_Template.BP_Up1_Template_C" (Math|Transform|MakeTransform (Transformation|GetWorldLocation (Variables|Default|GetSpawnLocationLane0)) "0, 0, 0" "1,1,1") "Undefined" 0 0))
      (CallFunction|AddTemplatetoArrayandCarryonVariables _returnvalue))
    (:1
      (bind _returnvalue_2 (Game|SpawnActorfromClass "/Game/CrimsonMaze/Core/LevelTemplates/Up/BP_Up2_Template.BP_Up2_Template_C" (Math|Transform|MakeTransform (Transformation|GetWorldLocation (Variables|Default|GetSpawnLocationLane0)) "0, 0, 0" "1,1,1") "Undefined" 0 0))
      (CallFunction|AddTemplatetoArrayandCarryonVariables _returnvalue_2))
    (:2
      (bind _returnvalue_3 (Game|SpawnActorfromClass "/Game/CrimsonMaze/Core/LevelTemplates/Up/BP_Up3_Template.BP_Up3_Template_C" (Math|Transform|MakeTransform (Transformation|GetWorldLocation (Variables|Default|GetSpawnLocationLane0)) "0, 0, 0" "1,1,1") "Undefined" 0 0))
      (CallFunction|AddTemplatetoArrayandCarryonVariables _returnvalue_3))))

(fn SpawnStraightandDownTemplate
  (Variables|Default|SetStraightLaneCount 0)
  ;[1 1 1] Weil danach 2 Lanes kommen
  (Variables|Default|SetSpawnInLane-1 true)
  (Variables|Default|SetSpawnInLane0 true)
  (switch int (Math|Random|RandomInteger 2)
    (:0
      (bind _returnvalue (Game|SpawnActorfromClass "/Game/CrimsonMaze/Core/LevelTemplates/Straight-Down/BP_StraightDown1_Template.BP_StraightDown1_Template_C" (Math|Transform|MakeTransform (Transformation|GetWorldLocation (Variables|Default|GetSpawnLocationLane0)) "0, 0, 0" "1,1,1") "Undefined" 0 0))
      (CallFunction|AddTemplatetoArrayandCarryonVariables _returnvalue))
    (:1
      (bind _returnvalue_2 (Game|SpawnActorfromClass "/Game/CrimsonMaze/Core/LevelTemplates/Straight-Down/BP_StraightDown2_Template.BP_StraightDown2_Template_C" (Math|Transform|MakeTransform (Transformation|GetWorldLocation (Variables|Default|GetSpawnLocationLane0)) "0, 0, 0" "1,1,1") "Undefined" 0 0))
      (CallFunction|AddTemplatetoArrayandCarryonVariables _returnvalue_2))))

(fn SpawnStraightandUpTemplate
  (Variables|Default|SetStraightLaneCount 0)
  (Variables|Default|SetSpawnInLane1 true)
  (Variables|Default|SetSpawnInLane0 true)
  (switch int (Math|Random|RandomInteger 2)
    (:0
      (bind _returnvalue (Game|SpawnActorfromClass "/Game/CrimsonMaze/Core/LevelTemplates/Straight-Up/BP_StraightUp1_Template.BP_StraightUp1_Template_C" (Math|Transform|MakeTransform (Transformation|GetWorldLocation (Variables|Default|GetSpawnLocationLane0)) "0, 0, 0" "1,1,1") "Undefined" 0 0))
      (CallFunction|AddTemplatetoArrayandCarryonVariables _returnvalue))
    (:1
      (bind _returnvalue_2 (Game|SpawnActorfromClass "/Game/CrimsonMaze/Core/LevelTemplates/Straight-Up/BP_StraightUp2_Template.BP_StraightUp2_Template_C" (Math|Transform|MakeTransform (Transformation|GetWorldLocation (Variables|Default|GetSpawnLocationLane0)) "0, 0, 0" "1,1,1") "Undefined" 0 0))
      (CallFunction|AddTemplatetoArrayandCarryonVariables _returnvalue_2))))

(fn SpawnStraightandUpandDownTemplate
  (Variables|Default|SetStraightLaneCount 0)
  (Variables|Default|SetSpawnInLane1 true)
  (Variables|Default|SetSpawnInLane-1 true)
  (Variables|Default|SetSpawnInLane0 true)
  (bind _returnvalue (Game|SpawnActorfromClass "/Game/CrimsonMaze/Core/LevelTemplates/Straight-Up-Down/BP_StraightUpDown1_Template.BP_StraightUpDown1_Template_C" (Math|Transform|MakeTransform (Transformation|GetWorldLocation (Variables|Default|GetSpawnLocationLane0)) "0, 0, 0" "1,1,1") "Undefined" 0 0))
  (CallFunction|AddTemplatetoArrayandCarryonVariables _returnvalue))

(fn SpawnUpandDownTemplate
  (Variables|Default|SetStraightLaneCount 0)
  ;[1 1 1] Hier ist Lane 0 ungültig!
  (Variables|Default|SetSpawnInLane1 true)
  (Variables|Default|SetSpawnInLane-1 true)
  (bind _returnvalue (Game|SpawnActorfromClass "/Game/CrimsonMaze/Core/LevelTemplates/Up-Down/BP_UpDown1_Template.BP_UpDown1_Template_C" (Math|Transform|MakeTransform (Transformation|GetWorldLocation (Variables|Default|GetSpawnLocationLane0)) "0, 0, 0" "1,1,1") "Undefined" 0 0))
  (CallFunction|AddTemplatetoArrayandCarryonVariables _returnvalue))